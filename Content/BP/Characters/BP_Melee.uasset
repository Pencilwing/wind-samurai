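; BP_Melee is a short-lived melee hit actor that damages BP_Pandit enemies overlapping its box, then destroys itself after a close-range hit or a brief delay.
; ProcessHit lowers the enemy's Life through ModifyEnemyHealth, which also updates the enemy hearts on BP_Blue's HUD.
; A lethal hit changes the enemy's state and hides the hearts; otherwise AddKnockBack launches it along X away from the player before another state change.
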(event OnComponentBeginOverlap(Box)
  (params (OverlappedComponent :type Primitive%20Component%20Object%20Reference) (OtherActor :type Actor%20Object%20Reference) (OtherComp :type Primitive%20Component%20Object%20Reference) (OtherBodyIndex :type Integer) (bFromSweep :type Boolean) (SweepResult :type Hit%20Result%20Structure%20%28by%20ref%29))
  (bind _asbp_pandit (Utilities|Casting|CastToBP_Pandit OtherActor))
  (if (<= (Transformation|GetDistanceTo _asbp_pandit) 2e+02)
    (CallFunction|ProcessHit _asbp_pandit)
    (Actor|DestroyActor)))

(event EventBeginPlay
  (Utilities|FlowControl|Delay 0.1)
  (Actor|DestroyActor))

(event Collision|EventHit
  (params (MyComp :type Primitive%20Component%20Object%20Reference) (Other :type Actor%20Object%20Reference) (OtherComp :type Primitive%20Component%20Object%20Reference) (bSelfMoved :type Boolean) (HitLocation :type Vector :default "0, 0, 0") (HitNormal :type Vector :default "0, 0, 0") (NormalImpulse :type Vector :default "0, 0, 0") (Hit :type Hit%20Result%20Structure%20%28by%20ref%29)))

(event EventTick
  (params (DeltaSeconds :type Float%20%28single-precision%29)))

(fn ConstructionScript)

(fn ProcessHit
  (params (PandaRef :type BP%20Pandit%20Object%20Reference))
  (if (not (Variables|/Game/BP/Characters/BP_Pandit.BP_Pandit_C|GetIsDead PandaRef))
    (bind _updatedhealth (CallFunction|ModifyEnemyHealth -1 PandaRef))
    (if (<= _updatedhealth 0)
      (Default|ChangeState PandaRef "NewEnumerator3")
      (bind _asbp_blue (Utilities|Casting|CastToBP_Blue (Game|GetPlayerCharacter 0)))
      (Widget|SetVisibility (Variables|/Game/VisualAssets/UI/HealthUI/GameHUD.GameHUD_C|GetEnemyHeartWrapBox (Variables|/Game/BP/Characters/BP_Blue.BP_Blue_C|GetHealthHUD _asbp_blue)) "Hidden")
      (return true)
      (else
        (CallFunction|AddKnockBack PandaRef)
        (Default|ChangeState PandaRef "NewEnumerator4")
        (return false)))))

(fn ModifyEnemyHealth
  (params (InputHealth :type Integer) (PandaRef :type BP%20Pandit%20Object%20Reference))
  (bind _output_get (Variables|/Game/BP/Characters/BP_Pandit.BP_Pandit_C|SetLife PandaRef (Math|Conversions|ToFloat(Integer) (+ (Math|Float|Truncate (Variables|/Game/BP/Characters/BP_Pandit.BP_Pandit_C|GetLife PandaRef)) (* InputHealth 25)))))
  (bind _asbp_blue (Utilities|Casting|CastToBP_Blue (Game|GetPlayerCharacter 0)))
  (Default|UpdateEnemyHeartHealth (Variables|/Game/BP/Characters/BP_Blue.BP_Blue_C|GetHealthHUD _asbp_blue) InputHealth)
  (return (Math|Float|Truncate _output_get)))

(fn AddKnockBack
  (params (Enemy :type Character%20Object%20Reference))
  (if (> (.x (Transformation|GetActorLocation Enemy)) (.x (Transformation|GetActorLocation (Game|GetPlayerCharacter 0))))
    (Character|LaunchCharacter Enemy "700.000000, 0, 0" true false)
    (else
      (Character|LaunchCharacter Enemy "-700.000000, 0, 0" true false))))