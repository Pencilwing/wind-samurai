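; BP_Blue is a 2D side-view flipbook character with platform-fighter style movement: crouch-windup jumps with shorthop, double jump, fast fall and a count-limited directional dash.
; Tick refreshes velocity-derived state flags, which a function-based state machine maps to a flipbook; the sprite flips through X scale.
; Dash launches along normalized input while gravity and friction are zeroed, then damps velocity after a delay; landing resets the dash count.
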(event Custom|UpdateAnim
  ;[1 1 1] Update Animation
  (Utilities|StateChecks)
  (bind _outputfb (CallFunction|AnimationStateMachine (Variables|Default|GetIsMoving) (Variables|Default|GetIsFalling) (Variables|Default|GetIsJumpCrouching) (Variables|Default|GetIsJumping) (Variables|Default|GetIsAttacking1)))
  (Sprite|SetFlipbook (Variables|Default|GetSprite) _outputfb))

(event EventTick
  (params (DeltaSeconds :type Float%20%28single-precision%29))
  ;[1 1 1] Event Tick
  (if (Variables|Default|GetIsDashing)
    (Variables|/Script/Engine.CharacterMovementComponent|SetGravityScale (Variables|Character|GetCharacterMovement) 0.0))
  (CallFunction|UpdateAnim)
  (if (not (Utilities|AirCheck))
    (Utilities|FlipCharacter)))

(event EventOnLanded
  (params (Hit :type Hit%20Result%20Structure%20%28by%20ref%29))
  ;[1 1 1] Movement Control
  ;;[1 1 1] Dash
  ;;;[1 1 1] Reset Dash Count
  (Variables|Default|SetDashCount 0))

(event Input|ActionEvents|InputActionJump
  (params (Key :type Key%20Structure))
  (bind _jumpcurrentcount (Variables|Default|GetJumpCurrentCount))
  (bind _returnvalue (<= _jumpcurrentcount 1))
  ;[1 1 1] Movement Control
  ;;[1 1 1] Jump, Double Jump and Shorthop
  (:Pressed
    (Character|StopJumping)
    (if (Utilities|AirCheck) ; Jump - Shorthop Window
      (Variables|Default|SetIsJumpCrouching false :!label _label)
      (if _returnvalue ; Jump
        (Character|Jump)
        (if (and _returnvalue (Utilities|AirCheck))
          (Variables|/Script/Engine.CharacterMovementComponent|SetJumpZVelocity (Variables|Character|GetCharacterMovement) (Variables|Default|GetJumpTwoStrength))
          (else
            (Variables|/Script/Engine.CharacterMovementComponent|SetJumpZVelocity (Variables|Character|GetCharacterMovement) (Variables|Default|GetJumpOneStrength)))))
      (else
        (Variables|Default|SetIsJumpCrouching true)
        (Utilities|FlowControl|Delay (Variables|Default|GetJumpCrouchTimeMax))
        (if (Variables|Default|GetIsJumpCrouching)
          (goto _label)))))
  (:Released
    (if (Utilities|AirCheck) ; Shorthop
      (Character|StopJumping)
      (else
        (Variables|Default|SetIsJumpCrouching false)
        (Variables|/Script/Engine.CharacterMovementComponent|SetJumpZVelocity (Variables|Character|GetCharacterMovement) (Variables|Default|GetJumpCrouchStrength))
        (Development|PrintString "JC JUMP")
        (Character|Jump)))))

(event Input|ActionEvents|InputActionJump
  (params (Key :type Key%20Structure))
  ;[1 1 1] Event Tick
  (:Pressed
    (Math|Integer|CompareInt (Variables|Default|GetJumpCurrentCount) (Variables|Default|GetJumpMaxCount)
      (:<
        (Utilities|FlipCharacter)))))

(event Input|ActionEvents|InputActionDash
  (params (Key :type Key%20Structure))
  ;[1 1 1] Movement Control
  ;;[1 1 1] Dash
  (:Pressed
    (if (Variables|Default|GetIsDashing)
      (if (not (>= (Variables|Default|GetDashCount) (Variables|Default|GetDashMax)))
        (if (!= (+ (Math|Float|Power (Input|AxisValues|GetMoveRight) 2.0) (Math|Float|Power (Input|AxisValues|GetUpDown) 2.0)) 0.0) :!label _label
          (Utilities|Dash
            (:OUT
              (Variables|Default|SetIsDashing false)))))
      (elif (not (>= (Variables|Default|GetDashCount) (Variables|Default|GetDashMax)))
        (goto _label)))))

(event Input|ActionEvents|InputActionFastFall
  (params (Key :type Key%20Structure))
  ;[1 1 1] Movement Control
  ;;[1 1 1] fastfall
  (:Pressed
    (if (Variables|Default|GetIsFalling)
      (if (not (Variables|Default|GetIsDashing))
        (Variables|/Script/Engine.CharacterMovementComponent|SetGravityScale (Variables|Character|GetCharacterMovement) (Variables|Default|GetFastFallSpeed))))))

(event Input|AxisEvents|InputAxisMoveRight
  (params (AxisValue :type Float%20%28single-precision%29))
  ;[1 1 1] Movement Control
  ;;[1 1 1] Horizontal Movement
  (Pawn|Input|AddMovementInput "1.000000,0.000000, 0" AxisValue false))

(event Input|AxisEvents|InputAxisMoveRight
  (params (AxisValue :type Float%20%28single-precision%29))
  ;[1 1 1] Event Tick
  (if (not (Variables|Default|GetIsDashing))
    (if (not (Utilities|AirCheck))
      (Utilities|FlipCharacter))))

(fn ConstructionScript)

(fn AnimationStateMachine
  (params (IsMoving :type Boolean) (IsFalling :type Boolean) (IsJumpCrouching :type Boolean) (IsJumping :type Boolean) (IsAttacking1 :type Boolean))
  (if IsFalling
    (LocalVariables|SetAnimationState "NewEnumerator3")
    (return (Utilities|Select :Index (LocalVariables|GetAnimationState) :NewEnumerator0 "/Game/VisualAssets/Characters/Blue/FB_Blue_test_Idle.FB_Blue_test_Idle" :NewEnumerator1 "/Game/VisualAssets/Characters/Blue/FB_Blue_test_run.FB_Blue_test_run" :NewEnumerator2 "/Game/VisualAssets/Characters/Blue/FB_Blue_test_jumping.FB_Blue_test_jumping" :NewEnumerator3 "/Game/VisualAssets/Characters/Blue/FB_Blue_test_falling.FB_Blue_test_falling" :NewEnumerator4 "/Game/VisualAssets/Characters/Blue/FB_Blue_test_jumpcrouch.FB_Blue_test_jumpcrouch" :NewEnumerator5 "/Game/VisualAssets/Characters/Blue/FB_Blue_test_Idle.FB_Blue_test_Idle"))
    (elif IsJumping
      (LocalVariables|SetAnimationState "NewEnumerator2")
      (return (Utilities|Select :Index (LocalVariables|GetAnimationState) :NewEnumerator0 "/Game/VisualAssets/Characters/Blue/FB_Blue_test_Idle.FB_Blue_test_Idle" :NewEnumerator1 "/Game/VisualAssets/Characters/Blue/FB_Blue_test_run.FB_Blue_test_run" :NewEnumerator2 "/Game/VisualAssets/Characters/Blue/FB_Blue_test_jumping.FB_Blue_test_jumping" :NewEnumerator3 "/Game/VisualAssets/Characters/Blue/FB_Blue_test_falling.FB_Blue_test_falling" :NewEnumerator4 "/Game/VisualAssets/Characters/Blue/FB_Blue_test_jumpcrouch.FB_Blue_test_jumpcrouch" :NewEnumerator5 "/Game/VisualAssets/Characters/Blue/FB_Blue_test_Idle.FB_Blue_test_Idle"))
      (elif IsJumpCrouching
        (LocalVariables|SetAnimationState "NewEnumerator4")
        (return (Utilities|Select :Index (LocalVariables|GetAnimationState) :NewEnumerator0 "/Game/VisualAssets/Characters/Blue/FB_Blue_test_Idle.FB_Blue_test_Idle" :NewEnumerator1 "/Game/VisualAssets/Characters/Blue/FB_Blue_test_run.FB_Blue_test_run" :NewEnumerator2 "/Game/VisualAssets/Characters/Blue/FB_Blue_test_jumping.FB_Blue_test_jumping" :NewEnumerator3 "/Game/VisualAssets/Characters/Blue/FB_Blue_test_falling.FB_Blue_test_falling" :NewEnumerator4 "/Game/VisualAssets/Characters/Blue/FB_Blue_test_jumpcrouch.FB_Blue_test_jumpcrouch" :NewEnumerator5 "/Game/VisualAssets/Characters/Blue/FB_Blue_test_Idle.FB_Blue_test_Idle"))
        (elif IsMoving
          (LocalVariables|SetAnimationState "NewEnumerator1")
          (return (Utilities|Select :Index (LocalVariables|GetAnimationState) :NewEnumerator0 "/Game/VisualAssets/Characters/Blue/FB_Blue_test_Idle.FB_Blue_test_Idle" :NewEnumerator1 "/Game/VisualAssets/Characters/Blue/FB_Blue_test_run.FB_Blue_test_run" :NewEnumerator2 "/Game/VisualAssets/Characters/Blue/FB_Blue_test_jumping.FB_Blue_test_jumping" :NewEnumerator3 "/Game/VisualAssets/Characters/Blue/FB_Blue_test_falling.FB_Blue_test_falling" :NewEnumerator4 "/Game/VisualAssets/Characters/Blue/FB_Blue_test_jumpcrouch.FB_Blue_test_jumpcrouch" :NewEnumerator5 "/Game/VisualAssets/Characters/Blue/FB_Blue_test_Idle.FB_Blue_test_Idle"))
          (elif IsAttacking1
            (LocalVariables|SetAnimationState "NewEnumerator5")
            (else
              (LocalVariables|SetAnimationState "NewEnumerator0")
              (return (Utilities|Select :Index (LocalVariables|GetAnimationState) :NewEnumerator0 "/Game/VisualAssets/Characters/Blue/FB_Blue_test_Idle.FB_Blue_test_Idle" :NewEnumerator1 "/Game/VisualAssets/Characters/Blue/FB_Blue_test_run.FB_Blue_test_run" :NewEnumerator2 "/Game/VisualAssets/Characters/Blue/FB_Blue_test_jumping.FB_Blue_test_jumping" :NewEnumerator3 "/Game/VisualAssets/Characters/Blue/FB_Blue_test_falling.FB_Blue_test_falling" :NewEnumerator4 "/Game/VisualAssets/Characters/Blue/FB_Blue_test_jumpcrouch.FB_Blue_test_jumpcrouch" :NewEnumerator5 "/Game/VisualAssets/Characters/Blue/FB_Blue_test_Idle.FB_Blue_test_Idle")))))))))

(fn DebugPrintScreen)

(fn FallingCheck
  (bind _output_get (Variables|Default|SetIsFalling (and (< (.Z (Math|Vector|BreakVector (Transformation|GetVelocity))) 0.0) (AI|Components|NavMovement|IsFalling (Variables|Character|GetCharacterMovement)))))
  (if (not _output_get)
    (Variables|/Script/Engine.CharacterMovementComponent|SetGravityScale (Variables|Character|GetCharacterMovement) 1.0)))

(fn JumpingCheck
  (Variables|Default|SetIsJumping (and (> (.Z (Math|Vector|BreakVector (Transformation|GetVelocity))) 0.0) (AI|Components|NavMovement|IsFalling (Variables|Character|GetCharacterMovement))))
  (if (and (AI|Components|NavMovement|IsFalling (Variables|Character|GetCharacterMovement)) (> (Math|Vector|VectorLength (Transformation|GetVelocity)) 5e+02))
    _))

(fn MovingCheck
  (bind _returnvalue (Transformation|GetVelocity))
  (bind _returnvalue_2 (Transformation|GetVelocity))
  (bind _x (Math|Vector|BreakVector _returnvalue_2))
  (bind _returnvalue_3 (< _x 0.0))
  (bind _returnvalue_4 (> _x 0.0))
  (Variables|Default|SetIsMoving (or _returnvalue_4 _returnvalue_3))
  (Variables|Default|SetIsMovingRight _returnvalue_4)
  (Variables|Default|SetIsMovingLeft _returnvalue_3)
  (if (< (Math|Vector|VectorLength (Transformation|GetVelocity)) 2e+01)
    (Variables|/Script/Engine.MovementComponent|SetVelocity (Variables|Character|GetCharacterMovement) (Math|Vector|MakeVector 0.0 (.y _returnvalue) (.z _returnvalue)))))

(fn JumpCrouchCheck)