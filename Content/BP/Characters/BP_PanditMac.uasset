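; Pandit Mac NPC whose paper sprite paces horizontally within 100 units of its start X, moved each Tick.
; BeginPlay assigns the Mac heist scene to BPDialogueBoxComponent, and inner and outer trigger overlaps with BP_Blue are forwarded to that component.
; FlipsOff only prints a message.
; Box layout and text helper functions are present but uncalled here, with several disconnected calculations.
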(event OnComponentBeginOverlap(InTrigger)
  (params (OverlappedComponent :type Primitive%20Component%20Object%20Reference) (OtherActor :type Actor%20Object%20Reference) (OtherComp :type Primitive%20Component%20Object%20Reference) (OtherBodyIndex :type Integer) (bFromSweep :type Boolean) (SweepResult :type Hit%20Result%20Structure%20%28by%20ref%29))
  (Utilities|Casting|CastToBP_Blue OtherActor)
  (Default|InTriggerOverlapStart (Variables|Default|GetBP_DialogueBoxComponent)))

(event OnComponentEndOverlap(InTrigger)
  (params (OverlappedComponent :type Primitive%20Component%20Object%20Reference) (OtherActor :type Actor%20Object%20Reference) (OtherComp :type Primitive%20Component%20Object%20Reference) (OtherBodyIndex :type Integer))
  (Utilities|Casting|CastToBP_Blue OtherActor)
  (Default|InTriggerOverlapEnd (Variables|Default|GetBP_DialogueBoxComponent)))

(event OnComponentEndOverlap(OutTrigger)
  (params (OverlappedComponent :type Primitive%20Component%20Object%20Reference) (OtherActor :type Actor%20Object%20Reference) (OtherComp :type Primitive%20Component%20Object%20Reference) (OtherBodyIndex :type Integer))
  (Utilities|Casting|CastToBP_Blue OtherActor)
  (Default|OutTriggerOverlapEnd (Variables|Default|GetBP_DialogueBoxComponent)))

(event Custom|FlipsOff
  (Development|PrintString "LeGasp You made it work"))

(event EventBeginPlay
  (Variables|Default|SetInitialLocation (.x (Transformation|GetWorldLocation (Variables|Default|GetPaperSprite))))
  (CallFunction|GetCharacterCurrentScene)
  (Variables|/Game/BP/DialogueSystem/BP_DialogueBoxComponent.BP_DialogueBoxComponent_C|SetCharacterCurrentScene (Variables|Default|GetBP_DialogueBoxComponent) (Variables|Default|GetMacCurrentScene)))

(event EventTick
  (params (DeltaSeconds :type Float%20%28single-precision%29))
  (bind _papersprite (Variables|Default|GetPaperSprite))
  (bind _papersprite_2 (Variables|Default|GetPaperSprite))
  (bind _returnvalue (Transformation|GetWorldLocation _papersprite))
  (bind _returnvalue_2 (Transformation|GetWorldLocation _papersprite_2))
  (if (Variables|Default|GetMovingLeft)
    (Math|Float|CompareFloat (.x _returnvalue) (- (Variables|Default|GetInitialLocation) 1e+02)
      (:>
        (Transformation|SetWorldLocation (Variables|Default|GetPaperSprite) (Math|Vector|MakeVector (+ (.x _returnvalue) -1.0) (.y _returnvalue) (.z _returnvalue)) false false))
      (:==
        (Variables|Default|SetMovingLeft false :!label _label))
      (:<
        (goto _label)))
    (else
      (Math|Float|CompareFloat (.x _returnvalue_2) (+ (Variables|Default|GetInitialLocation) 1e+02)
        (:>
          (Variables|Default|SetMovingLeft true :!label _label_2))
        (:==
          (goto _label_2))
        (:<
          (Transformation|SetWorldLocation (Variables|Default|GetPaperSprite) (Math|Vector|MakeVector (+ (.x _returnvalue_2) 1.0) (.y _returnvalue_2) (.z _returnvalue_2)) false false))))))

(event Custom|GetCharacterCurrentScene
  (Variables|Default|SetMacCurrentScene (Variables|Default|GetSCN_MacHeist1)))

(fn ConstructionScript)