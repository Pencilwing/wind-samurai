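; BP_Enemy_Melee is a short-lived enemy melee hitbox that damages the BP_Blue player and destroys itself after a brief delay on BeginPlay.
; A Box overlap with BP_Blue within range runs ProcessHit, then destroys the hitbox immediately.
; ProcessHit lowers player health and updates the heart HUD through ModifyHealth, destroying the player at zero.
; AddKnockBack does nothing because its launch logic is disconnected, and ModifyEnemyHealth is never called here.
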(event OnComponentBeginOverlap(Box)
  (params (OverlappedComponent :type Primitive%20Component%20Object%20Reference) (OtherActor :type Actor%20Object%20Reference) (OtherComp :type Primitive%20Component%20Object%20Reference) (OtherBodyIndex :type Integer) (bFromSweep :type Boolean) (SweepResult :type Hit%20Result%20Structure%20%28by%20ref%29))
  (bind _asbp_blue (Utilities|Casting|CastToBP_Blue OtherActor))
  (if (<= (Transformation|GetDistanceTo _asbp_blue) 2e+02)
    (CallFunction|ProcessHit)
    (Actor|DestroyActor)))

(event EventBeginPlay
  (Utilities|FlowControl|Delay 0.1)
  (Actor|DestroyActor))

(event EventTick
  (params (DeltaSeconds :type Float%20%28single-precision%29)))

(fn ConstructionScript)

(fn ProcessHit
  (params (PandaRef :type BP%20Pandit%20Object%20Reference))
  (bind _remaininghealth (CallFunction|ModifyHealth -1))
  (if (<= _remaininghealth 0)
    (Actor|DestroyActor (Game|GetPlayerCharacter 0))
    (else
      (CallFunction|AddKnockBack))))

(fn ModifyEnemyHealth
  (params (InputHealth :type Integer) (PandaRef :type BP%20Pandit%20Object%20Reference))
  (bind _output_get (Variables|/Game/BP/Characters/BP_Pandit.BP_Pandit_C|SetLife PandaRef (Math|Conversions|ToFloat(Integer) (+ (Math|Float|Truncate (Variables|/Game/BP/Characters/BP_Pandit.BP_Pandit_C|GetLife PandaRef)) (* InputHealth 25)))))
  (bind _asbp_blue (Utilities|Casting|CastToBP_Blue (Game|GetPlayerCharacter 0)))
  (Default|UpdateEnemyHeartHealth (Variables|/Game/BP/Characters/BP_Blue/BP_Blue.BP_Blue_C|GetHealthHUD _asbp_blue) InputHealth)
  (return (Math|Float|Truncate _output_get)))

(fn AddKnockBack
  (params (Enemy :type Character%20Object%20Reference)))

(fn ModifyHealth
  (params (InputHealth :type Integer))
  (bind _asbp_blue (Utilities|Casting|CastToBP_Blue (Game|GetPlayerCharacter 0)))
  (bind _output_get (Variables|/Game/BP/Characters/BP_Blue/BP_Blue.BP_Blue_C|SetHealth _asbp_blue (+ (Variables|/Game/BP/Characters/BP_Blue/BP_Blue.BP_Blue_C|GetHealth _asbp_blue) (* InputHealth 25))))
  (Default|UpdateHeartHealth (Variables|/Game/BP/Characters/BP_Blue/BP_Blue.BP_Blue_C|GetHealthHUD _asbp_blue) InputHealth)
  (return _output_get))