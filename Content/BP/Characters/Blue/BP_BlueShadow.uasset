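; BP_BlueShadow is a Paper2D sprite drop shadow that follows the Blue character.
; Each tick it traces down on the Camera channel from BlueActor, taken from a global variable, ignoring that actor.
; On a hit, it places the sprite just above the surface and shrinks it linearly with distance, down to MinimumSize.
; With no hit, the sprite is hidden.
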(event EventBeginPlay
  (bind _output (CallFunction|GetGlobalVar))
  (Utilities|Array|Add (Variables|Default|GetIgnoreObjects) (Variables|/Game/BP/GlobalBlueprints/BP_GameController.BP_GameController_C|GetBlueActor _output)))

(event EventTick
  (params (DeltaSeconds :type Float%20%28single-precision%29))
  (bind _papersprite (Variables|Default|GetPaperSprite))
  (bind _minimumsize (Variables|Default|GetMinimumSize))
  (bind (_outhit _returnvalue) (Collision|LineTraceByChannel (Math|Vector|MakeVector (.x (Transformation|GetActorLocation (Variables|/Game/BP/GlobalBlueprints/BP_GameController.BP_GameController_C|GetBlueActor (stale EventBeginPlay _output)))) (.y (Transformation|GetActorLocation (Variables|/Game/BP/GlobalBlueprints/BP_GameController.BP_GameController_C|GetBlueActor (stale EventBeginPlay _output)))) (.z (Transformation|GetActorLocation (Variables|/Game/BP/GlobalBlueprints/BP_GameController.BP_GameController_C|GetBlueActor (stale EventBeginPlay _output))))) (Math|Vector|MakeVector (.x (Transformation|GetActorLocation (Variables|/Game/BP/GlobalBlueprints/BP_GameController.BP_GameController_C|GetBlueActor (stale EventBeginPlay _output)))) (.y (Transformation|GetActorLocation (Variables|/Game/BP/GlobalBlueprints/BP_GameController.BP_GameController_C|GetBlueActor (stale EventBeginPlay _output)))) -5e+03) "TraceTypeQuery2" false (Variables|Default|GetIgnoreObjects) "None"))
  (if _returnvalue
    (Rendering|SetVisibility (Variables|Default|GetPaperSprite) true false)
    (if (< (+ (* (.distance _outhit) -0.001) 0.59) (Variables|Default|GetMinimumSize))
      (Transformation|SetWorldTransform _papersprite (Math|Transform|MakeTransform (Math|Vector|MakeVector (.x (Transformation|GetActorLocation (Variables|/Game/BP/GlobalBlueprints/BP_GameController.BP_GameController_C|GetBlueActor (stale EventBeginPlay _output)))) (.y (Transformation|GetActorLocation (Variables|/Game/BP/GlobalBlueprints/BP_GameController.BP_GameController_C|GetBlueActor (stale EventBeginPlay _output)))) (+ (.z (.location _outhit)) 1.0)) "0, 0, 0" (Math|Vector|MakeVector _minimumsize 1.0 _minimumsize)) false false)
      (else
        (Transformation|SetWorldTransform _papersprite (Math|Transform|MakeTransform (Math|Vector|MakeVector (.x (Transformation|GetActorLocation (Variables|/Game/BP/GlobalBlueprints/BP_GameController.BP_GameController_C|GetBlueActor (stale EventBeginPlay _output)))) (.y (Transformation|GetActorLocation (Variables|/Game/BP/GlobalBlueprints/BP_GameController.BP_GameController_C|GetBlueActor (stale EventBeginPlay _output)))) (+ (.z (.location _outhit)) 1.0)) "0, 0, 0" (Math|Vector|MakeVector (+ (* (.distance _outhit) -0.001) 0.59) 1.0 (+ (* (.distance _outhit) -0.001) 0.59))) false false)))
    (else
      (Rendering|SetVisibility (Variables|Default|GetPaperSprite) false false))))

(fn ConstructionScript)