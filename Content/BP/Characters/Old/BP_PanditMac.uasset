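; Pandit Mac, a Paper2D sprite character that paces side to side around its start X and hosts dialogue for BP_Blue.
; Tick drives the patrol and, on a trace hit with the player nearby, latches detection and last position without changing movement.
; Inner and outer triggers notify BPDialogueBoxComponent, whose scene is set to SCNMacHeist1 at BeginPlay.
; FlipsOff and Hit only print; the layout helper graphs look unfinished.
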(event OnComponentBeginOverlap(InTrigger)
  (params (OverlappedComponent :type Primitive%20Component%20Object%20Reference) (OtherActor :type Actor%20Object%20Reference) (OtherComp :type Primitive%20Component%20Object%20Reference) (OtherBodyIndex :type Integer) (bFromSweep :type Boolean) (SweepResult :type Hit%20Result%20Structure%20%28by%20ref%29))
  (Utilities|Casting|CastToBP_Blue OtherActor)
  (Default|InTriggerOverlapStart (Variables|Default|GetBP_DialogueBoxComponent)))

(event OnComponentEndOverlap(InTrigger)
  (params (OverlappedComponent :type Primitive%20Component%20Object%20Reference) (OtherActor :type Actor%20Object%20Reference) (OtherComp :type Primitive%20Component%20Object%20Reference) (OtherBodyIndex :type Integer))
  (Utilities|Casting|CastToBP_Blue OtherActor)
  (Default|InTriggerOverlapEnd (Variables|Default|GetBP_DialogueBoxComponent)))

(event OnComponentEndOverlap(OutTrigger)
  (params (OverlappedComponent :type Primitive%20Component%20Object%20Reference) (OtherActor :type Actor%20Object%20Reference) (OtherComp :type Primitive%20Component%20Object%20Reference) (OtherBodyIndex :type Integer))
  (Utilities|Casting|CastToBP_Blue OtherActor)
  (Default|OutTriggerOverlapEnd (Variables|Default|GetBP_DialogueBoxComponent)))

(event Custom|FlipsOff
  (Development|PrintString "LeGasp You made it work"))

(event Collision|EventHit
  (params (MyComp :type Primitive%20Component%20Object%20Reference) (Other :type Actor%20Object%20Reference) (OtherComp :type Primitive%20Component%20Object%20Reference) (bSelfMoved :type Boolean) (HitLocation :type Vector :default "0, 0, 0") (HitNormal :type Vector :default "0, 0, 0") (NormalImpulse :type Vector :default "0, 0, 0") (Hit :type Hit%20Result%20Structure%20%28by%20ref%29))
  (Development|PrintString "Hello"))

(event EventBeginPlay
  (Variables|Default|SetInitialLocation (.x (Transformation|GetWorldLocation (Variables|Default|GetPaperSprite))))
  (CallFunction|GetCharacterCurrentScene)
  (Variables|/Game/BP/DialogueSystem/BP_DialogueBoxComponent.BP_DialogueBoxComponent_C|SetCharacterCurrentScene (Variables|Default|GetBP_DialogueBoxComponent) (Variables|Default|GetMacCurrentScene)))

(event EventTick
  (params (DeltaSeconds :type Float%20%28single-precision%29))
  (bind _returnvalue (Transformation|GetActorLocation))
  (bind _returnvalue_2 (Game|GetPlayerCharacter 0))
  (bind _papersprite (Variables|Default|GetPaperSprite))
  (bind _papersprite_2 (Variables|Default|GetPaperSprite))
  (bind _returnvalue_3 (Transformation|GetWorldLocation _papersprite))
  (bind _returnvalue_4 (Transformation|GetWorldLocation _papersprite_2))
  (bind _returnvalue_5 (Transformation|GetActorLocation _returnvalue_2))
  (if (Variables|Default|GetPayerDetected)
    _
    (else
      (bind _returnvalue_6 (Collision|LineTraceByChannel _returnvalue _returnvalue_5 "TraceTypeQuery1" true 0 "ForDuration" true "(R=1.000000,G=0.000000,B=0.000000,A=1.000000)" "(R=0.000000,G=1.000000,B=0.000000,A=1.000000)" 0.2))))
  (if _returnvalue_6
    (if (< (Math|Vector|VectorLength (- _returnvalue _returnvalue_5)) 2.4e+02)
      (Variables|Default|SetPayerDetected true)
      (Variables|Default|SetPlayerLastPosition (Transformation|GetActorLocation (Game|GetPlayerCharacter 0)))))
  (if (Variables|Default|GetMovingLeft)
    (Math|Float|CompareFloat (.x _returnvalue_3) (- (Variables|Default|GetInitialLocation) 1e+02)
      (:>
        (Transformation|SetWorldLocation (Variables|Default|GetPaperSprite) (Math|Vector|MakeVector (+ (.x _returnvalue_3) -1.0) (.y _returnvalue_3) (.z _returnvalue_3)) false false))
      (:==
        (Variables|Default|SetMovingLeft false :!label _label))
      (:<
        (goto _label)))
    (else
      (Math|Float|CompareFloat (.x _returnvalue_4) (+ (Variables|Default|GetInitialLocation) 1e+02)
        (:>
          (Variables|Default|SetMovingLeft true :!label _label_2))
        (:==
          (goto _label_2))
        (:<
          (Transformation|SetWorldLocation (Variables|Default|GetPaperSprite) (Math|Vector|MakeVector (+ (.x _returnvalue_4) 1.0) (.y _returnvalue_4) (.z _returnvalue_4)) false false))))))

(event Custom|GetCharacterCurrentScene
  (Variables|Default|SetMacCurrentScene (Variables|Default|GetSCN_MacHeist1)))

(fn ConstructionScript)