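; BP_BlueShadow is a blob shadow actor that projects a paper sprite onto the ground beneath the Blue character.
; Each tick it line traces from the character, fetched through a global variable lookup, straight down on the Camera channel.
; On a hit, the sprite sits just above the impact point and shrinks with distance down to a minimum size.
; With no hit, the sprite is hidden.
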(event EventBeginPlay
  (bind _output (CallFunction|GetGlobalVar)))

(event EventTick
  (params (DeltaSeconds :type Float%20%28single-precision%29))
  (bind _papersprite (Variables|Default|GetPaperSprite))
  (bind _blueactor (Variables|Default|GetBlueActor))
  (bind _minimumsize (Variables|Default|GetMinimumSize))
  (bind _blueactor_2 (Variables|Default|GetBlueActor))
  (bind _returnvalue (Transformation|GetActorLocation _blueactor_2))
  (bind _returnvalue_2 (Transformation|GetActorLocation _blueactor))
  (bind (_outhit _returnvalue_3) (Collision|LineTraceByChannel (Math|Vector|MakeVector (.x (Transformation|GetActorLocation (Variables|/Game/BP/GlobalBlueprints/BP_GameController.BP_GameController_C|GetBlueActor (stale EventBeginPlay _output)))) (.y (Transformation|GetActorLocation (Variables|/Game/BP/GlobalBlueprints/BP_GameController.BP_GameController_C|GetBlueActor (stale EventBeginPlay _output)))) (.z (Transformation|GetActorLocation (Variables|/Game/BP/GlobalBlueprints/BP_GameController.BP_GameController_C|GetBlueActor (stale EventBeginPlay _output))))) (Math|Vector|MakeVector (.x (Transformation|GetActorLocation (Variables|/Game/BP/GlobalBlueprints/BP_GameController.BP_GameController_C|GetBlueActor (stale EventBeginPlay _output)))) (.y (Transformation|GetActorLocation (Variables|/Game/BP/GlobalBlueprints/BP_GameController.BP_GameController_C|GetBlueActor (stale EventBeginPlay _output)))) -5e+03) "TraceTypeQuery2" false (Utilities|Array|MakeArray (Variables|/Game/BP/GlobalBlueprints/BP_GameController.BP_GameController_C|GetBlueActor (stale EventBeginPlay _output))) "None"))
  (if _returnvalue_3
    (Rendering|SetVisibility (Variables|Default|GetPaperSprite) true false)
    (if (< (+ (* (.distance _outhit) -0.001) 0.59) (Variables|Default|GetMinimumSize))
      (Transformation|SetWorldTransform _papersprite (Math|Transform|MakeTransform (Math|Vector|MakeVector (.x _returnvalue) (.y _returnvalue) (+ (.z (.location _outhit)) 1.0)) "0, 0, 0" (Math|Vector|MakeVector _minimumsize 1.0 _minimumsize)) false false)
      (else
        (Transformation|SetWorldTransform _papersprite (Math|Transform|MakeTransform (Math|Vector|MakeVector (.x _returnvalue_2) (.y _returnvalue_2) (+ (.z (.location _outhit)) 1.0)) "0, 0, 0" (Math|Vector|MakeVector (+ (* (.distance _outhit) -0.001) 0.59) 1.0 (+ (* (.distance _outhit) -0.001) 0.59))) false false)))
    (else
      (Rendering|SetVisibility (Variables|Default|GetPaperSprite) false false))))

(fn ConstructionScript)