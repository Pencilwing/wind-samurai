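; BP_Pandit is a 2D Paper enemy that fights the player and also hosts a dialogue box driven by BP_Blue trigger overlaps.
; A Tick-driven state machine moves it through idle wander, chase, charge attack, attack, knock and death, using pawn sensing and line-of-sight traces.
; Charging snapshots the player's position; attacking spawns BP_Enemy_Melee there, knocking back an unmoved player or showing game over at zero health.
; State flags select the flipbook each tick.
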(event OnComponentBeginOverlap(InTrigger)
  (params (OverlappedComponent :type Primitive%20Component%20Object%20Reference) (OtherActor :type Actor%20Object%20Reference) (OtherComp :type Primitive%20Component%20Object%20Reference) (OtherBodyIndex :type Integer) (bFromSweep :type Boolean) (SweepResult :type Hit%20Result%20Structure%20%28by%20ref%29))
  ;[1 1 1] Dialogue System
  (Utilities|Casting|CastToBP_Blue OtherActor)
  (Default|InTriggerOverlapStart (Variables|Default|GetBP_DialogueBoxComponent)))

(event OnComponentEndOverlap(OutTrigger)
  (params (OverlappedComponent :type Primitive%20Component%20Object%20Reference) (OtherActor :type Actor%20Object%20Reference) (OtherComp :type Primitive%20Component%20Object%20Reference) (OtherBodyIndex :type Integer))
  ;[1 1 1] Dialogue System
  (Utilities|Casting|CastToBP_Blue OtherActor)
  (Default|OutTriggerOverlapEnd (Variables|Default|GetBP_DialogueBoxComponent)))

(event OnComponentEndOverlap(InTrigger)
  (params (OverlappedComponent :type Primitive%20Component%20Object%20Reference) (OtherActor :type Actor%20Object%20Reference) (OtherComp :type Primitive%20Component%20Object%20Reference) (OtherBodyIndex :type Integer))
  ;[1 1 1] Dialogue System
  (Utilities|Casting|CastToBP_Blue OtherActor)
  (Default|InTriggerOverlapEnd (Variables|Default|GetBP_DialogueBoxComponent)))

(event OnSeePawn(PawnSensing)
  (params (Pawn :type Pawn%20Object%20Reference))
  ;[1 1 1] Idle State
  (Utilities|Casting|CastToPaperCharacter Pawn)
  (if (CallFunction|PathCleartoPlayer)
    (Utilities|FlowControl|Gate true) ; enters at Open
  ))

(event Custom|Close%20Chase%20Gate
  ;[1 1 1] Idle State
  (Utilities|FlowControl|Gate true) ; enters at Close
)

(event Custom|ResetAttack
  (bind _returnvalue (Game|GetPlayerCharacter 0))
  ;[1 1 1] Attack
  (Utilities|FlowControl|DoOnce false) ; enters at Reset
)

(event Custom|FlipsOff
  ;[1 1 1] Dialogue System
  (Development|PrintString "LeGasp You made it work"))

(event Custom|ResetChargeAttack
  ;[1 1 1] Charge Attack
  (Utilities|FlowControl|DoOnce false) ; enters at Reset
)

(event Custom|UpdateAnim
  (bind _outputfb (CallFunction|AnimationStateMachine (Variables|Default|GetIsDead) (Variables|Default|GetIsKnocked) (Variables|Default|GetIsAttacking) (Variables|Default|GetIsChasing)))
  (Sprite|SetFlipbook (Variables|Default|GetPaperFlipbook) _outputfb))

(event Custom|ResetIdle
  (bind _returnvalue (Transformation|GetActorLocation))
  (bind _randomlocation (AI|Navigation|GetRandomReachablePointinRadius _returnvalue 2e+02))
  ;[1 1 1] Idle
  (Utilities|FlowControl|DoOnce false) ; enters at Reset
)

(event Custom|Idle
  (bind _returnvalue (Transformation|GetActorLocation))
  (bind _randomlocation (AI|Navigation|GetRandomReachablePointinRadius _returnvalue 2e+02))
  ;[1 1 1] Idle
  (Utilities|FlowControl|DoOnce false
    (:Completed
      (Variables|Default|SetIsIdle true)
      (AI|AIMoveTo self (Math|Vector|MakeVector (.x _randomlocation) 0.0 (.z _randomlocation)) 0 5.0 true
        (:then
          (Utilities|FlowControl|Delay (Variables|Default|GetidleStop%28secs%29))
          (CallFunction|ResetIdle))))))

(event Custom|ChargeAttack
  ;[1 1 1] Charge Attack
  (Utilities|FlowControl|DoOnce false
    (:Completed
      (Variables|Default|SetIsAttacking true)
      (Variables|Default|SetIsChasing false)
      (Variables|Default|SetIsIdle false)
      (if (Variables|Default|GetHasPlayerPosition)
        _
        (else
          (Variables|Default|SetPlayerPosition (Transformation|GetActorLocation (Game|GetPlayerCharacter 0)))
          (Variables|Default|SetHasPlayerPosition true)))
      (CallFunction|ResetChargeAttack))))

(event Custom|Dead
  ;[1 1 1] Dead
  (Utilities|FlowControl|DoOnce false
    (:Completed
      (Variables|Default|SetIsDead true)
      (Components|DestroyComponent (Variables|Default|GetOutTrigger))
      (Components|DestroyComponent (Variables|Default|GetInTrigger))
      (Components|DestroyComponent (Variables|Default|GetBP_DialogueBoxComponent)))))

(event Custom|Chase
  ;[1 1 1] Chase
  (Variables|Default|SetIsChasing true)
  (Variables|Default|SetIsKnocked false)
  (Variables|Default|SetIsAttacking false)
  (Variables|Default|SetIsIdle false)
  (AI|Navigation|SimpleMovetoActor (AI|GetAIController self) (Variables|Default|GetplayerRef)))

(event Custom|Knock
  ;[1 1 1] Knocked
  (Utilities|FlowControl|DoOnce false
    (:Completed
      (Variables|Default|SetIsKnocked true)
      (Variables|Default|SetIsAttacking false)
      (Variables|Default|SetIsIdle false)
      (Variables|Default|SetIsChasing false)
      (CallFunction|ResetKnock))))

(event Custom|ResetKnock
  ;[1 1 1] Knocked
  (Utilities|FlowControl|DoOnce false) ; enters at Reset
)

(event Custom|Attack
  (bind _returnvalue (Game|GetPlayerCharacter 0))
  ;[1 1 1] Attack
  (Utilities|FlowControl|DoOnce false
    (:Completed
      (Variables|Default|SetHasPlayerPosition false)
      (bind _asbp_blue (Utilities|Casting|CastToBP_Blue (Game|GetPlayerCharacter 0)))
      (Game|SpawnActorfromClass "/Game/BP/Characters/BP_Enemy_Melee.BP_Enemy_Melee_C" (Math|Transform|MakeTransform (Variables|Default|GetPlayerPosition) (Transformation|GetActorRotation self) (Transformation|GetActorScale3D self)) "Undefined" 0 0)
      (Utilities|IsValid _asbp_blue
        (:Is%20Valid
          (Variables|/Game/BP/Characters/Blue/BP_Blue.BP_Blue_C|SetHealthCounter _asbp_blue 0.0)
          (Variables|Default|SetAttackCounter 0.0)
          (if (<= (Variables|/Game/BP/Characters/Blue/BP_Blue.BP_Blue_C|GetHealth _asbp_blue) 0)
            (CallFunction|ShowGameOverMenu :!label _label)
            (else
              (if (Math|Vector|Equal(Vector) (Variables|Default|GetPlayerPosition) (Transformation|GetActorLocation (Game|GetPlayerCharacter 0)) 0.0001)
                (CallFunction|AddKnockback)
                (Input|DisableInput _returnvalue 0)
                (Utilities|FlowControl|Delay 0.2)
                (Input|EnableInput _returnvalue 0))
              (CallFunction|ResetAttack))))
        (:Is%20Not%20Valid
          (goto _label))))))

(event EventTick
  (params (DeltaSeconds :type Float%20%28single-precision%29))
  (bind _returnvalue (Transformation|GetActorLocation))
  (Utilities|FlowControl|Sequence
    (:then_0
      (switch Utilities|FlowControl|Switch|SwitchonENUM_ai_states (Variables|Default|Getstates)
        (:NewEnumerator0
          (CallFunction|Idle)
          ;[1 1 1] Idle State
          (Utilities|FlowControl|Gate true
            (:Exit
              (CallFunction|ChangeState "NewEnumerator1"))))
        (:NewEnumerator1
          (CallFunction|Chase)
          ;[1 1 1] Chase State
          (Utilities|FlowControl|Sequence
            (:then_0
              (CallFunction|CloseChaseGate))
            (:then_1
              (if (<= (CallFunction|GetDistancetoPlayer) (Variables|Default|GetattackDistance))
                (CallFunction|ChangeState "NewEnumerator5")
                (elif (not (CallFunction|PathCleartoPlayer))
                  (Utilities|FlowControl|Delay (Variables|Default|GetgiveUpTime%28secs%29))
                  (if (not (CallFunction|PathCleartoPlayer))
                    (CallFunction|ChangeState "NewEnumerator0")))))))
        (:NewEnumerator2
          (CallFunction|Attack)
          ;[1 1 1] Attack State
          (CallFunction|CloseChaseGate)
          (if (or (> (CallFunction|GetDistancetoPlayer) (Variables|Default|GetattackDistance)) (not (CallFunction|PathCleartoPlayer)))
            _
            (else
              _))
          (CallFunction|ChangeState "NewEnumerator1"))
        (:NewEnumerator3
          (CallFunction|Dead))
        (:NewEnumerator4
          ;[1 1 1] Knock State
          (CallFunction|Knock)
          (Utilities|FlowControl|Delay 0.1)
          (if (> (Variables|Default|GetLife) 0.0)
            (Variables|Default|Setstates "NewEnumerator1")
            (else
              (Variables|Default|Setstates "NewEnumerator3"))))
        (:NewEnumerator5
          ;[1 1 1] Charge Attack State
          (CallFunction|ChargeAttack)
          (Utilities|FlowControl|Delay 0.4)
          (if (> (Variables|Default|GetLife) 0.0)
            (if (Variables|Default|GetIsKnocked)
              (CallFunction|ChangeState "NewEnumerator4")
              (else
                (CallFunction|ChangeState "NewEnumerator2")))
            (else
              (CallFunction|ChangeState "NewEnumerator3"))))))
    (:then_1
      (Development|PrintString (Utilities|String|EnumtoString (Variables|Default|Getstates)) true true "(R=0.000000,G=0.660000,B=1.000000,A=1.000000)" DeltaSeconds))
    (:then_2
      (CallFunction|FlipPanda)
      (Transformation|SetActorLocation (Math|Vector|MakeVector (.x _returnvalue) 0.0 (.z _returnvalue)) false false))
    (:then_3
      (CallFunction|UpdateAttackCounter)
      (CallFunction|UpdateAnim))))

(event EventBeginPlay
  ;[1 1 1] Begin Play
  (bind _aspaper_character (Utilities|Casting|CastToPaperCharacter (Game|GetPlayerCharacter 0)))
  (Variables|Default|SetplayerRef _aspaper_character)
  (CallFunction|GetCharacterCurrentScene)
  (Variables|/Game/BP/DialogueSystem/BP_DialogueBoxComponent.BP_DialogueBoxComponent_C|SetCharacterCurrentScene (Variables|Default|GetBP_DialogueBoxComponent) (Variables|Default|GetMacCurrentScene)))

(event Custom|GetCharacterCurrentScene
  (Variables|Default|SetMacCurrentScene (Variables|Default|GetSCN_MacHeist1)))

(fn ConstructionScript)

(fn PathCleartoPlayer
  (bind _playerref (Variables|Default|GetplayerRef))
  (Utilities|IsValid _playerref
    (:Is%20Valid
      (bind _outhit (Collision|LineTraceByChannel (Transformation|GetActorLocation) (Transformation|GetActorLocation _playerref) "TraceTypeQuery2" false 0 "None"))
      (Utilities|Casting|CastToPaperCharacter (.HitActor (Collision|BreakHitResult _outhit))
        (:then
          (return true))
        (:CastFailed
          (return false))))))

(fn ChangeState
  (params (newState :type ENUM_ai_states%20Enum :default "NewEnumerator0"))
  (Class|NavMovementComponent|StopActiveMovement (Variables|Character|GetCharacterMovement))
  (Variables|Default|Setstates newState)
  (CallFunction|ResetIdle)
  (CallFunction|ResetAttack))

(fn GetDistancetoPlayer
  (bind _returnvalue (Transformation|GetActorLocation))
  (bind _playerref (Variables|Default|GetplayerRef))
  (bind _returnvalue_2 (Transformation|GetActorLocation _playerref))
  (Utilities|IsValid _playerref
    (:Is%20Valid
      (return (Math|Float|Sqrt (+ (Math|Float|Square (- (.x _returnvalue_2) (.x _returnvalue))) (Math|Float|Square (- (.z _returnvalue_2) (.z _returnvalue)))))))))

(fn ShowGameOverMenu
  (Game|SetGamePaused true)
  (Utilities|IsValid (Variables|Default|GetGameOverMenu)
    (:Is%20Valid
      _)
    (:Is%20Not%20Valid
      (bind _returnvalue (UserInterface|CreateWidget "/Game/BP/UI/UI_Menus/BP_GameOverMenu.BP_GameOverMenu_C" (Game|GetPlayerController 0)))
      (bind _output_get (Variables|Default|SetGameOverMenu _returnvalue))))
  (UserInterface|Viewport|AddtoViewport (Variables|Default|GetGameOverMenu) 0)
  (Input|SetInputModeUIOnly (Game|GetPlayerController 0) (Variables|/Game/BP/UI/UI_Menus/BP_MenuButton.BP_MenuButton_C|GetMyButton (Variables|/Game/BP/UI/UI_Menus/BP_GameOverMenu.BP_GameOverMenu_C|GetBP_MenuButtonRetry _output_get)) "DoNotLock")
  (Variables|/Script/Engine.PlayerController|SetbShowMouseCursor (Game|GetPlayerController 0) true))

(fn FlipPanda
  (bind _output (CallFunction|GetGlobalVar))
  (if (> (.x (Transformation|GetActorForwardVector)) 0.0)
    (Transformation|SetActorRotation (Math|Rotator|MakeRotator 0.0 0.0 0.0))
    (Variables|/Game/BP/GlobalBlueprints/BP_GameController.BP_GameController_C|SetPandaFlip _output false)
    (else
      (Transformation|SetActorRotation (Math|Rotator|MakeRotator 0.0 0.0 1.8e+02))
      (Variables|/Game/BP/GlobalBlueprints/BP_GameController.BP_GameController_C|SetPandaFlip _output true))))

(fn AddKnockback
  (if (> (.x (Transformation|GetActorLocation)) (.x (Transformation|GetActorLocation (Game|GetPlayerCharacter 0))))
    (Character|LaunchCharacter (Game|GetPlayerCharacter 0) "-800.000000, 0, 0" true false)
    (else
      (Character|LaunchCharacter (Game|GetPlayerCharacter 0) "800.000000, 0, 0" true false))))

(fn UpdateAttackCounter
  (Variables|Default|SetAttackCounter (+ (Variables|Default|GetAttackCounter) 1.0)))

(fn AnimationStateMachine
  (params (IsDead :type Boolean) (IsKnocked :type Boolean) (IsAttacking :type Boolean) (IsChasing :type Boolean))
  (if IsDead
    (Variables|Default|SetAnimationStates "NewEnumerator4")
    (Development|PrintString "1")
    (elif IsKnocked
      (Variables|Default|SetAnimationStates "NewEnumerator3")
      (Development|PrintString "2")
      (elif IsAttacking
        (Variables|Default|SetAnimationStates "NewEnumerator1")
        (Development|PrintString "3")
        (elif IsChasing
          (Variables|Default|SetAnimationStates "NewEnumerator2")
          (Development|PrintString "4")
          (else
            (Variables|Default|SetAnimationStates "NewEnumerator0")
            (Development|PrintString "5"))))))
  (return (Utilities|Select :Index (Variables|Default|GetAnimationStates) :NewEnumerator0 "/Game/VisualAssets/Characters/Pandit_Mac/PanditFlipbooks/FB_Pandit_Idle.FB_Pandit_Idle" :NewEnumerator1 "/Game/VisualAssets/Characters/Pandit_Mac/PanditFlipbooks/FB_Pandit_Attack.FB_Pandit_Attack" :NewEnumerator2 "/Game/VisualAssets/Characters/Pandit_Mac/PanditFlipbooks/FB_Pandit_Run.FB_Pandit_Run" :NewEnumerator3 0 :NewEnumerator4 0)))