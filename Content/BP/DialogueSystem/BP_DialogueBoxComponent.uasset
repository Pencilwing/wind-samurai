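; Dialogue component that shows a BP_DialogueBox above its owning actor and toggles scenes in response to inner and outer trigger overlap events.
; Inner overlap start sets the global scene and visibility, spawns and attaches the box, then toggles BP_SceneController, guarded by a DoOnce.
; Inner exit tears down only while the controller's scene is inactive, outer exit only while active.
; Teardown hides and toggles the scene, destroys the box and re-arms spawning.
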(event Custom|InTriggerOverlapStart
  (Utilities|FlowControl|DoOnce false
    (:Completed
      (bind _outactors (Actor|GetAllActorsOfClass "/Game/BP/DialogueSystem/BP_SceneController.BP_SceneController_C"))
      (Variables|Default|SetSceneController (Utilities|Array|Get(acopy) _outactors))
      (bind _output (CallFunction|GetGlobalVar))
      (Variables|/Game/BP/GlobalBlueprints/BP_GameController.BP_GameController_C|SetsceneVisible _output true)
      (Variables|/Game/BP/GlobalBlueprints/BP_GameController.BP_GameController_C|SetcurrentScene _output (Variables|Default|GetCharacterCurrentScene))
      (bind _returnvalue (Game|SpawnActorfromClass "/Game/BP/DialogueSystem/BP_DialogueBox.BP_DialogueBox_C" (Math|Transform|MakeTransform "0, 0, 0") "AdjustIfPossibleButAlwaysSpawn" 0 0))
      (Variables|Default|SetLocalDialogueBox _returnvalue)
      (Transformation|AttachActorToActor _returnvalue (Components|GetOwner) "None" "KeepRelative" "KeepWorld" "KeepWorld" false)
      (Transformation|SetActorRelativeLocation _returnvalue "0,3.000000,120.000000")
      (Default|ToggleScene (Variables|Default|GetSceneController)))))

(event Custom|Reset%20DialogueSpawn
  (Utilities|FlowControl|DoOnce false) ; enters at Reset
)

(event Custom|InTriggerOverlapEnd
  (bind _output (CallFunction|GetGlobalVar))
  (if (Variables|/Game/BP/GlobalBlueprints/BP_GameController.BP_GameController_C|GetsceneVisible _output)
    (if (not (Variables|/Game/BP/DialogueSystem/BP_SceneController.BP_SceneController_C|GetsceneActive (Variables|Default|GetSceneController)))
      (bind _output_2 (CallFunction|GetGlobalVar))
      (Variables|/Game/BP/GlobalBlueprints/BP_GameController.BP_GameController_C|SetsceneVisible _output_2 false)
      (Default|ToggleScene (Variables|Default|GetSceneController))
      (Actor|DestroyActor (Variables|Default|GetLocalDialogueBox))
      (CallFunction|ResetDialogueSpawn))))

(event Custom|OutTriggerOverlapEnd
  (bind _localdialoguebox (Variables|Default|GetLocalDialogueBox))
  (if (Variables|/Game/BP/DialogueSystem/BP_SceneController.BP_SceneController_C|GetsceneActive (Variables|Default|GetSceneController))
    (bind _output (CallFunction|GetGlobalVar))
    (Variables|/Game/BP/GlobalBlueprints/BP_GameController.BP_GameController_C|SetsceneVisible _output false)
    (Default|ToggleScene (Variables|Default|GetSceneController))
    (if (Utilities|IsValid _localdialoguebox)
      (Actor|DestroyActor _localdialoguebox)
      (CallFunction|ResetDialogueSpawn))))

(event EventBeginPlay)