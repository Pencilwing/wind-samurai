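; World-space dialogue box that resizes to fit the current dialogue text from BP_SceneController.
; DialogueEvent sets visible and sizing text, waits briefly, then derives box dimensions from measured text bounds, padding and corner size.
; It scales side and center pieces nine-slice style, snaps corners and sides to the box edges, then positions the arrow relative to a side piece.
; Tick holds the container's world rotation at zero.
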(event Custom|DialogueEvent
  (bind _translength (Utilities|TransformLength))
  (bind _transheight (Utilities|TransformHeight))
  (bind _center_0__0_ (Variables|Default|GetCenter%200,%200%20))
  (bind _side_1__0 (Variables|Default|GetSide%201,%200))
  (bind _side__1__0 (Variables|Default|GetSide%20-1,%200))
  (bind _side_0__1 (Variables|Default|GetSide%200,%201))
  (bind _side_0___1 (Variables|Default|GetSide%200,%20-1))
  (bind _center_0__0__2 (Variables|Default|GetCenter%200,%200%20))
  ;[1 1 1] Define Text and Sizes
  (Utilities|SetVariables)
  ;[1 1 1] Scale Parts
  (Transformation|SetRelativeScale3D (Variables|Default|GetSide%200,%201) (Math|Vector|MakeVector (/ _translength (/ (.Length (Utilities|GetHeightLength _side_0__1)) (.x (Variables|/Script/Engine.SceneComponent|GetRelativeScale3D _side_0__1)))) 1.0 1.0))
  (Transformation|SetRelativeScale3D (Variables|Default|GetSide%200,%20-1) (Math|Vector|MakeVector (/ _translength (/ (.Length (Utilities|GetHeightLength _side_0___1)) (.x (Variables|/Script/Engine.SceneComponent|GetRelativeScale3D _side_0___1)))) 1.0 -1.0))
  (Transformation|SetRelativeScale3D (Variables|Default|GetSide%201,%200) (Math|Vector|MakeVector -1.0 1.0 (/ _transheight (/ (.Height (Utilities|GetHeightLength _side_1__0)) (.z (Variables|/Script/Engine.SceneComponent|GetRelativeScale3D _side_1__0))))))
  (Transformation|SetRelativeScale3D (Variables|Default|GetSide%20-1,%200) (Math|Vector|MakeVector 1.0 1.0 (/ _transheight (/ (.Height (Utilities|GetHeightLength _side__1__0)) (.z (Variables|/Script/Engine.SceneComponent|GetRelativeScale3D _side__1__0))))))
  (Transformation|SetRelativeScale3D (Variables|Default|GetCenter%200,%200%20) (Math|Vector|MakeVector (/ (Utilities|TransformLength) (/ (.Length (Utilities|GetHeightLength _center_0__0__2)) (.x (Variables|/Script/Engine.SceneComponent|GetRelativeScale3D _center_0__0__2)))) 1.0 (/ (Utilities|TransformHeight) (/ (.Height (Utilities|GetHeightLength _center_0__0_)) (.z (Variables|/Script/Engine.SceneComponent|GetRelativeScale3D _center_0__0_))))))
  ;[1 1 1] Position Parts
  (Utilities|SetPositions (Variables|Default|GetCorner%20-1,%201) (Variables|Default|GetSide%20-1,%200) (Variables|Default|GetCorner%20-1,%20-1) "left" ; SetLeft
    (:Completed
      (Utilities|SetPositions (Variables|Default|GetCorner%201,%20-1) (Variables|Default|GetSide%201,%200) (Variables|Default|GetCorner%201,%201) "right" ; SetRIght
        (:Completed
          (Utilities|SetPositions (Variables|Default|GetCorner%20-1,%201) (Variables|Default|GetSide%200,%201) (Variables|Default|GetCorner%201,%201) "up" ; SetUp
            (:Completed
              (Utilities|SetPositions (Variables|Default|GetCorner%201,%20-1) (Variables|Default|GetSide%200,%20-1) (Variables|Default|GetCorner%20-1,%20-1) "down" ; SetDown
                (:Completed
                  (Transformation|SetRelativeLocation (Variables|Default|GetDialogueArrow) (Math|Vector|MakeVector 5.0 5.0 (- (.z (Variables|/Script/Engine.SceneComponent|GetRelativeLocation (Variables|Default|GetSide%200,%20-1))) (.Height (Utilities|GetHeightLength (Variables|Default|GetSide%200,%20-1))))) false true))))))))))

(event EventBeginPlay
  (bind _outactors (Actor|GetAllActorsOfClass "/Game/BP/DialogueSystem/BP_SceneController.BP_SceneController_C"))
  (Variables|Default|SetSceneController (Utilities|Array|Get(acopy) _outactors)))

(event EventTick
  (params (DeltaSeconds :type Float%20%28single-precision%29))
  (Transformation|SetWorldRotation (Variables|Default|GetDialogueBoxContainer) "0,0.000000, 0" false false))

(event Input|ActionEvents|InputActionDebugButton
  (params (Key :type Key%20Structure))
  ;[1 1 1] Debug
  (:Pressed
    (Development|PrintString (Utilities|String|ToString(Float) (.x (.BoxExtent (Collision|GetComponentBounds (Variables|Default|GetTextSize))))))))

(fn ConstructionScript)