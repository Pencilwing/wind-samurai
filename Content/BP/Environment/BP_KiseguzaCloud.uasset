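; A drifting background cloud actor for the Kiseguza sky, drawn with a Paper2D sprite.
; On BeginPlay it picks a random drift speed and one of the first two sprites in its cloud array.
; Each Tick moves it along +X by that speed without delta-time scaling.
; Past a fixed X limit it destroys itself and asks the first BP_KiseguzaSky found to generate a replacement cloud.
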(event EventBeginPlay
  (Variables|Default|SetCloudSpeed (Math|Random|RandomFloatinRange 0.05 0.5))
  (Rendering|Components|Sprite|SetSprite (Variables|Default|GetPaperSprite) (Utilities|Array|Get(acopy) (Variables|Default|GetCloudsArray) (Math|Random|RandomIntegerinRange 0 1))))

(event EventTick
  (params (DeltaSeconds :type Float%20%28single-precision%29))
  (bind _papersprite (Variables|Default|GetPaperSprite))
  (bind _relativelocation (Variables|/Script/Engine.SceneComponent|GetRelativeLocation _papersprite))
  (if (> (.x _relativelocation) 1.08e+03)
    (Actor|DestroyActor)
    (bind _outactors (Actor|GetAllActorsOfClass "/Game/BP/Environment/BP_KiseguzaSky.BP_KiseguzaSky_C"))
    (Default|GenerateCloud (Utilities|Array|Get(acopy) _outactors))
    (else
      (Transformation|SetActorRelativeLocation (Math|Vector|MakeVector (+ (Variables|Default|GetCloudSpeed) (.x _relativelocation)) (.y _relativelocation) (.z _relativelocation))))))

(fn ConstructionScript)