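; BP_KiseguzaSky is a sky backdrop actor for a Paper2D scene that scatters clouds and follows BlueActor.
; On BeginPlay it spawns BP_KiseguzaCloud actors in a loop bounded by MaxClouds, at random X/Z points within a 1920x1080 area.
; Each cloud gets one of the first two CloudsArray sprites at random.
; Every Tick the sky copies BlueActor's X and Z, obtained through GetGlobalVar, while holding a fixed Y depth.
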(event EventBeginPlay
  (bind _output (CallFunction|GetGlobalVar))
  (for _index (range 0 (Variables|Default|GetMaxClouds))
    (bind _returnvalue (Game|SpawnActorfromClass "/Game/BP/Environment/BP_KiseguzaCloud.BP_KiseguzaCloud_C" (Math|Transform|MakeTransform (Math|Vector|MakeVector (Math|Random|RandomFloatinRange 0.0 1.92e+03) 0.0 (Math|Random|RandomFloatinRange 0.0 1.08e+03))) "Undefined" 0 0))
    (Rendering|Components|Sprite|SetSprite (Variables|/Game/BP/Environment/BP_KiseguzaCloud.BP_KiseguzaCloud_C|GetPaperSprite _returnvalue) (Utilities|Array|Get(acopy) (Variables|Default|GetCloudsArray) (Math|Random|RandomIntegerinRange 0 1)))))

(event EventTick
  (params (DeltaSeconds :type Float%20%28single-precision%29))
  (Transformation|SetActorLocation (Math|Vector|MakeVector (.x (Transformation|GetActorLocation (Variables|/Game/BP/GlobalBlueprints/BP_GameController.BP_GameController_C|GetBlueActor (stale EventBeginPlay _output)))) -5e+02 (.z (Transformation|GetActorLocation (Variables|/Game/BP/GlobalBlueprints/BP_GameController.BP_GameController_C|GetBlueActor (stale EventBeginPlay _output))))) false false))

(fn ConstructionScript)